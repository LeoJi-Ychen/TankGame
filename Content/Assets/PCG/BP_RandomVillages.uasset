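; Editor-time village scatterer that places random meshes on surfaces within the SpawnBounds box.
; The construction script destroys its static mesh components, then makes ten downward Visibility line traces between randomly sampled points.
; Each hit gets a mesh from Meshes with random per-axis scale, random yaw and a vertical ZOffset.
; Randomness is unseeded, so the layout changes whenever the script reruns.
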(event EventBeginPlay)

(event Collision|EventActorBeginOverlap
  (params (OtherActor :type Actor%20Object%20Reference)))

(event EventTick
  (params (DeltaSeconds :type Float%20%28single-precision%29)))

(fn ConstructionScript
  (bind _meshes (Variables|Default|GetMeshes))
  (bind _maxscale (Variables|Default|GetMaxScale))
  (bind _minscale (Variables|Default|GetMinScale))
  (bind _spawnbounds (Variables|Default|GetSpawnBounds))
  (bind _spawnbounds_2 (Variables|Default|GetSpawnBounds))
  (bind _returnvalue (Transformation|GetWorldLocation _spawnbounds))
  (bind _returnvalue_2 (Components|Box|GetScaledBoxExtent _spawnbounds_2))
  (bind _returnvalue_3 (Math|Random|RandomFloatinRange _minscale _maxscale))
  (bind _returnvalue_4 (Math|Random|RandomPointinBoundingBox _returnvalue _returnvalue_2))
  (bind (_x _y _z) (Math|Vector|BreakVector _returnvalue_4))
  (for _array_element (Actor|GetComponentsByClass "/Script/Engine.StaticMeshComponent")
    (Components|DestroyComponent _array_element))
  (for _index (range 0 9)
    (bind (_outhit _returnvalue_5) (Collision|LineTraceByChannel (Math|Vector|MakeVector _x _y (+ _z 3e+03)) (Math|Vector|MakeVector _x _y (- _z 1e+02)) "TraceTypeQuery1" false 0 "None"))
    (if _returnvalue_5
      (bind _returnvalue_6 (AddComponent|AddStaticMeshComponent false))
      (Components|StaticMesh|SetStaticMesh _returnvalue_6 (Utilities|Array|Get(acopy) _meshes (Math|Random|RandomIntegerinRange 0 (Utilities|Array|LastIndex _meshes))))
      (Transformation|SetWorldScale3D _returnvalue_6 (Math|Vector|MakeVector _returnvalue_3 _returnvalue_3 _returnvalue_3))
      (Transformation|SetWorldLocation _returnvalue_6 (Math|Vector|MakeVector (.X (Math|Vector|BreakVector (.Location (Collision|BreakHitResult _outhit)))) (.Y (Math|Vector|BreakVector (.Location (Collision|BreakHitResult _outhit)))) (+ (.Z (Math|Vector|BreakVector (.Location (Collision|BreakHitResult _outhit)))) (Variables|Default|GetZOffset))) false false)
      (Transformation|SetWorldRotation _returnvalue_6 (Math|Rotator|MakeRotator 0.0 0.0 (Math|Random|RandomFloatinRange 0.0 3.6e+02)) false false))))