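; Player-driven tank that moves, aims, fires and switches between two weapons through WeaponManager.
; Tick polls keys, pushing the physics hull TANKLOWER with forces, torque and extra downward force, then moves the actor to follow it.
; Mouse deltas from a cursor re-centred each frame rotate the turret and pitch the clamped Top.
; A UIHUD widget shows weapon highlight and speed read from TankEngineAudio; forward input activates dust effects.
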(event Custom|DustToggle
  (params (Ismoving :type Boolean))
  (if Ismoving
    (Components|Activation|Activate (Variables|Default|GetDust) false)
    (Components|Activation|Activate (Variables|Default|GetDust1) false)
    (else
      (Components|Activation|Deactivate (Variables|Default|GetDust))
      (Components|Activation|Deactivate (Variables|Default|GetDust1)))))

(event Collision|EventActorBeginOverlap
  (params (OtherActor :type Actor%20Object%20Reference)))

(event EventBeginPlay
  ;[1 1 1] HUD注释
  ;;[1 1 1] UIupload
  (Utilities|FlowControl|Sequence
    (:then_0
      (bind _returnvalue (UserInterface|CreateWidget "/Game/ui/UIHUD.UIHUD_C"))
      (bind _output_get (Variables|Default|SetHUD%20Ref _returnvalue))
      (UserInterface|Viewport|AddtoViewport _output_get 0)
      (Default|UpdateWeaponHighlight (Variables|Default|GetHUD%20Ref) 2 false))
    (:then_1
      (CallFunction|HideMouseCursor)
      (Class|PlayerController|SetMouseLocation (Game|GetPlayerController 0) 100 100))))

(event EventTick
  (params (DeltaSeconds :type Float%20%28single-precision%29))
  (bind _returnvalue (Game|GetPlayerController 0))
  (bind _returnvalue_2 (Game|GetPlayerController 0))
  (bind _tank_lower (Variables|Default|GetTANK_LOWER))
  (bind _tankengineaudio (Variables|Default|GetTankEngineAudio))
  (bind _top (Variables|Default|GetTop))
  (bind _tank_lower_2 (Variables|Default|GetTANK_LOWER))
  (bind _tank_lower_3 (Variables|Default|GetTANK_LOWER))
  (bind _top_2 (Variables|Default|GetTop))
  (bind _returnvalue_3 (Transformation|GetWorldLocation _tank_lower))
  (bind _returnvalue_4 (Class|TankEngineAudioComponent|GetCurrentSpeed _tankengineaudio))
  (bind _relativerotation (Variables|/Script/Engine.SceneComponent|GetRelativeRotation _top_2))
  (Utilities|FlowControl|Sequence
    (:then_2
      (Utilities|FlowControl|Sequence
        (:then_0
          ;[1 1 1] Tank movement
          (if (Game|Player|IsInputKeyDown _returnvalue "W")
            (Physics|AddForce _tank_lower_2 (* (Math|Vector|GetRightVector _tank_lower_2) 4e+04) "None" true)
            (CallFunction|DustToggle true)))
        (:then_1
          (if (Game|Player|IsInputKeyDown _returnvalue "S")
            (Physics|AddForce _tank_lower_3 (* (Math|Vector|GetRightVector _tank_lower_3) -3.5e+04) "None" true)))
        (:then_2
          (if (Game|Player|IsInputKeyDown _returnvalue "D")
            (Class|PrimitiveComponent|AddTorqueinDegrees (Variables|Default|GetTANK_LOWER) "0.000000,0.000000,500.000000" "None" true)))
        (:then_3
          (if (Game|Player|IsInputKeyDown _returnvalue "A")
            (Class|PrimitiveComponent|AddTorqueinDegrees (Variables|Default|GetTANK_LOWER) "0.000000,0.000000,-500.000000" "None" true)))))
    (:then_3
      ;[1 0 0.8208] Gravity
      (Physics|AddForce (Variables|Default|GetTANK_LOWER) "0.000000,0.000000,-30000.000000" "None" true))
    (:then_4
      ;[1 1 1] Shoot
      (if (Game|Player|IsInputKeyDown _returnvalue_2 "LeftMouseButton")
        (Class|WeaponManagerComponent|Fire (Variables|Default|GetWeaponManager) "0, 0, 0" "0, 0, 0")))
    (:then_5
      (Utilities|FlowControl|Sequence
        (:then_0
          (if (Game|Player|IsInputKeyDown _returnvalue_2 "One")
            (Class|WeaponManagerComponent|SwitchWeaponbyIndex (Variables|Default|GetWeaponManager))))
        (:then_1
          (if (Game|Player|IsInputKeyDown _returnvalue_2 "Two")
            (Class|WeaponManagerComponent|SwitchWeaponbyIndex (Variables|Default|GetWeaponManager) 1)))))
    (:then_6
      (CallFunction|GetMosueAxis)
      (Utilities|FlowControl|Sequence
        (:then_0
          (Transformation|AddRelativeRotation (Variables|Default|GetCube) (Math|Rotator|MakeRotator 0.0 0.0 (Variables|Default|Getx)) false false))
        (:then_1
          (Transformation|AddLocalRotation _top_2 (Math|Rotator|MakeRotator (Variables|Default|Gety) 0.0 0.0) false false)
          (if (< (.roll _relativerotation) -2e+01)
            (Transformation|SetRelativeRotation _top "0.000000,0.000000,-20.000000" false false)
            (elif (> (.roll _relativerotation) 1e+01)
              (Transformation|SetRelativeRotation _top "0.000000,0.000000,10.000000" false false))))))
    (:then_7
      (if (Utilities|Operators|NotEqual(!=) _returnvalue_3 (Transformation|GetActorLocation) 1.0)
        (Transformation|SetActorLocation _returnvalue_3 false false)
        (Transformation|SetWorldLocation _tank_lower _returnvalue_3 false false)))
    (:then_8
      (Progress|SetPercent (Variables|/Game/ui/UIHUD.UIHUD_C|Getspeedbar (Variables|Default|GetHUD%20Ref)) (Math|Float|MapRangeClamped _returnvalue_4 0.0 1e+03 0.0 1.0)))
    (:then_9
      (Rendering|Components|TextRender|SetText (Variables|/Game/ui/UIHUD.UIHUD_C|Getspeedtext (Variables|Default|GetHUD%20Ref)) (Utilities|Text|FormatText (Utilities|Text|ToText(Integer) (Math|Float|Round (Math|Float|MapRangeClamped _returnvalue_4 0.0 1e+03 0.0 6e+01))))))))

(event Input|KeyboardEvents|2
  (params (Key :type Key%20Structure :default "None"))
  ;[1 1 1] HUD注释
  ;;[1 1 1] keyboardCheck
  (:Pressed
    (Default|UpdateWeaponHighlight (Variables|Default|GetHUD%20Ref) 1 false)))

(event Input|KeyboardEvents|SpaceBar
  (params (Key :type Key%20Structure :default "None"))
  (:Pressed
    (if (Variables|/Script/Engine.PlayerController|GetbShowMouseCursor (Game|GetPlayerController 0))
      (Variables|/Script/Engine.PlayerController|SetbShowMouseCursor (Game|GetPlayerController 0) false)
      (else
        (Variables|/Script/Engine.PlayerController|SetbShowMouseCursor (Game|GetPlayerController 0) false)))))

(event Input|KeyboardEvents|1
  (params (Key :type Key%20Structure :default "None"))
  ;[1 1 1] HUD注释
  ;;[1 1 1] keyboardCheck
  (:Pressed
    (Default|UpdateWeaponHighlight (Variables|Default|GetHUD%20Ref) 2 false)))

(fn ConstructionScript)

(fn GetMosueAxis
  (bind _returnvalue (Game|GetPlayerController 0))
  (bind (_locationx _locationy) (Game|Player|GetMousePosition _returnvalue))
  (Variables|Default|Setx 0.0)
  (Variables|Default|Sety 0.0)
  (Utilities|FlowControl|Sequence
    (:then_0
      (Variables|Default|Setcmp_x _locationx)
      (if (!= _locationx 1e+02)
        (if (> (Math|Float|Absolute(Float) (- (Variables|Default|Getcmp_x) 1e+02)) 2.0)
          (Variables|Default|Setx (- (Variables|Default|Getcmp_x) 1e+02))
          (else
            (Variables|Default|Setx 0.0)))))
    (:then_1
      (Variables|Default|Setcmp_y _locationy)
      (if (!= _locationy 1e+02)
        (if (> (Math|Float|Absolute(Float) (- (Variables|Default|Getcmp_y) 1e+02)) 2.0)
          (Variables|Default|Sety (- (Variables|Default|Getcmp_y) 1e+02))
          (else
            (Variables|Default|Sety 0.0)))))
    (:then_2
      (Class|PlayerController|SetMouseLocation _returnvalue 100 100))))

(fn HideMouseCursor
  (Variables|/Script/Engine.PlayerController|SetbShowMouseCursor (Game|GetPlayerController 0) false))