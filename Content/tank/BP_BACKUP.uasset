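; Tank Blueprint, named as a backup, with mouse-aimed turret and keyboard movement, both polled every Tick from player controller 0.
; Gun yaws in world space toward the visibility-trace hit under the cursor, with pitch and roll held at zero.
; W/S and D/A push TANKLOWER with fixed world-space acceleration along X and vertical Z respectively, through an if/else chain allowing one key at a time.
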(event EventBeginPlay)

(event Collision|EventActorBeginOverlap
  (params (OtherActor :type Actor%20Object%20Reference)))

(event EventTick
  (params (DeltaSeconds :type Float%20%28single-precision%29))
  (bind _returnvalue (Game|GetPlayerController 0))
  (Utilities|FlowControl|Sequence
    (:then_0
      ;[0.1873 1 0.3294] Turret Movement
      (Transformation|SetWorldRotation (Variables|Default|Getgun%20) (Math|Rotator|MakeRotator 0.0 0.0 (.yaw (Math|Rotator|FindLookatRotation (Transformation|GetWorldLocation (Variables|Default|Getgun%20)) (.Location (Collision|BreakHitResult (.HitResult (Game|Player|GetHitResultUnderCursorbyChannel (Game|GetPlayerController 0) "TraceTypeQuery1" true))))))) false false))
    (:then_1
      ;[1 1 1] Tank movement
      (if (Game|Player|IsInputKeyDown _returnvalue "W")
        (Physics|AddForce (Variables|Default|GetTANK_LOWER) "-1000.000000,0.000000,0.000000" "None" true)
        (elif (Game|Player|IsInputKeyDown _returnvalue "S")
          (Physics|AddForce (Variables|Default|GetTANK_LOWER) "1000.000000,0.000000,0.000000" "None" true)
          (elif (Game|Player|IsInputKeyDown _returnvalue "D")
            (Physics|AddForce (Variables|Default|GetTANK_LOWER) "0.000000,0.000000,1000.000000" "None" true)
            (elif (Game|Player|IsInputKeyDown _returnvalue "A")
              (Physics|AddForce (Variables|Default|GetTANK_LOWER) "0.000000,0.000000,-1000.000000" "None" true))))))))

(fn ConstructionScript)