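; Player-controlled tank that drives on physics, aims its gun at the cursor and fires through a WeaponManager component.
; Tick polls keys directly: exclusive WASD force or torque on the lower hull, extra downward force, mouse firing and 1/2 weapon switching.
; BeginPlay creates the HUD, whose weapon highlight follows the number keys.
; TankEngineAudio's speed is printed as debug text, and Space only ever hides the cursor.
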(event Collision|EventActorBeginOverlap
  (params (OtherActor :type Actor%20Object%20Reference)))

(event EventBeginPlay
  ;[1 1 1] HUD注释
  ;;[1 1 1] UIupload
  (Utilities|FlowControl|Sequence
    (:then_0
      (bind _returnvalue (UserInterface|CreateWidget "/Game/hudsound/UIHUD.UIHUD_C"))
      (bind _output_get (Variables|Default|SetHUD%20Ref _returnvalue))
      (UserInterface|Viewport|AddtoViewport _output_get 0)
      (Default|UpdateWeaponHighlight (Variables|Default|GetHUD%20Ref) 2 false))))

(event EventTick
  (params (DeltaSeconds :type Float%20%28single-precision%29))
  (bind _returnvalue (Game|GetPlayerController 0))
  (bind _returnvalue_2 (Game|GetPlayerController 0))
  (bind _tank_lower (Variables|Default|GetTANK_LOWER))
  (bind _tank_lower_2 (Variables|Default|GetTANK_LOWER))
  (bind _tankengineaudio (Variables|Default|GetTankEngineAudio))
  (bind _returnvalue_3 (CallFunction|GetCurrentSpeed _tankengineaudio))
  (Utilities|FlowControl|Sequence
    (:then_0
      ;[0.1873 1 0.3294] Turret Movement
      (Transformation|SetWorldRotation (Variables|Default|Getgun%20) (Math|Rotator|MakeRotator 0.0 0.0 (.yaw (Math|Rotator|FindLookatRotation (Transformation|GetWorldLocation (Variables|Default|Getgun%20)) (.Location (Collision|BreakHitResult (.HitResult (Game|Player|GetHitResultUnderCursorbyChannel (Game|GetPlayerController 0) "TraceTypeQuery1" true))))))) false false))
    (:then_1
      ;[1 1 1] Tank movement
      (if (Game|Player|IsInputKeyDown _returnvalue "W")
        (Physics|AddForce _tank_lower (* (Math|Vector|GetRightVector _tank_lower) 5e+03) "None" true)
        (elif (Game|Player|IsInputKeyDown _returnvalue "S")
          (Physics|AddForce _tank_lower_2 (* (Math|Vector|GetRightVector _tank_lower_2) -5e+03) "None" true)
          (elif (Game|Player|IsInputKeyDown _returnvalue "D")
            (Class|PrimitiveComponent|AddTorqueinDegrees (Variables|Default|GetTANK_LOWER) "0.000000,0.000000,500.000000" "None" true)
            (elif (Game|Player|IsInputKeyDown _returnvalue "A")
              (Class|PrimitiveComponent|AddTorqueinDegrees (Variables|Default|GetTANK_LOWER) "0.000000,0.000000,-500.000000" "None" true))))))
    (:then_2
      ;[1 0 0.8208] Gravity
      (Physics|AddForce (Variables|Default|GetTANK_LOWER) "0.000000,0.000000,-3000.000000" "None" true))
    (:then_3
      ;[1 1 1] Shoot
      (if (Game|Player|IsInputKeyDown _returnvalue_2 "LeftMouseButton")
        (CallFunction|Fire (Variables|Default|GetWeaponManager) "0, 0, 0" "0, 0, 0")))
    (:then_4
      (Utilities|FlowControl|Sequence
        (:then_0
          (if (Game|Player|IsInputKeyDown _returnvalue_2 "One")
            (CallFunction|SwitchWeaponbyIndex (Variables|Default|GetWeaponManager))))
        (:then_1
          (if (Game|Player|IsInputKeyDown _returnvalue_2 "Two")
            (CallFunction|SwitchWeaponbyIndex (Variables|Default|GetWeaponManager) 1)))))
    (:then_5
      (Development|PrintString (Utilities|String|ToString(Text) (Utilities|Text|FormatText "Speed: {0}" _returnvalue_3)) true true "(R=0.000000,G=0.660000,B=1.000000,A=1.000000)" _returnvalue_3))))

(event Input|KeyboardEvents|2
  (params (Key :type Key%20Structure))
  ;[1 1 1] HUD注释
  ;;[1 1 1] keyboardCheck
  (:Pressed
    (Default|UpdateWeaponHighlight (Variables|Default|GetHUD%20Ref) 1 false)))

(event Input|KeyboardEvents|SpaceBar
  (params (Key :type Key%20Structure))
  (:Pressed
    (if (Variables|/Script/Engine.PlayerController|GetbShowMouseCursor (Game|GetPlayerController 0))
      (Variables|/Script/Engine.PlayerController|SetbShowMouseCursor (Game|GetPlayerController 0) false)
      (else
        (Variables|/Script/Engine.PlayerController|SetbShowMouseCursor (Game|GetPlayerController 0) false)))))

(event Input|KeyboardEvents|1
  (params (Key :type Key%20Structure))
  ;[1 1 1] HUD注释
  ;;[1 1 1] keyboardCheck
  (:Pressed
    (Default|UpdateWeaponHighlight (Variables|Default|GetHUD%20Ref) 2 false)))

(fn ConstructionScript)